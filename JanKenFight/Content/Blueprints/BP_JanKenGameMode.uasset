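; Game mode for a rock-paper-scissors duel where the player and a random enemy trade health damage each round.
; BeginPlay shows WBP_RPS_UI with UI-only input.
; OnPlayerChoice rolls the enemy's move with RandomInteger(2), which never yields scissors, then ResolveRound prints and damages the loser, though PlayerWins is never reset to false.
; CheckGameOver reopens NewMap when either health reaches zero, otherwise announces the next round.
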(event `self.ReceiveBeginPlay`
  (`self.StartRound`))

(fn `CheckGameOver`
  (if (<= (`self.PlayerHealth`) 0)
    (`KismetSystemLibrary.PrintString` "¡¡¡HAS PERDIDO!!!" true true (struct :`R` 1.0 :`B` 0.00479 :`A` 1.0) 5.0)
    (`GameplayStatics.OpenLevel` "NewMap")
    (elif (<= (`self.EnemyHealth`) 0)
      (`KismetSystemLibrary.PrintString` "¡¡¡HAS GANADO!!!" true true (struct :`R` 0.212641 :`G` 1.0 :`A` 1.0) 5.0)
      (`GameplayStatics.OpenLevel` "NewMap")
      (else
        (`KismetSystemLibrary.PrintString` "Siguiente ronda...")))))

(fn `OnPlayerChoice`
  (params (Choice :type Integer))
  (set `self.PlayerChoice` Choice)
  (set `self.EnemyChoice` (`KismetMathLibrary.RandomInteger` 2))
  (`self.ResolveRound`))

(fn `ResolveRound`
  (if (== (`self.PlayerChoice`) (`self.EnemyChoice`))
    (`KismetSystemLibrary.PrintString` "¡¡¡EMPATE!!!" true true (struct :`R` 1.0 :`G` 0.514501 :`A` 1.0) 5.0)
    (else
      (if (and (== (`self.PlayerChoice`) 0) (== (`self.EnemyChoice`) 2))
        (`KismetSystemLibrary.PrintString` "Piedra gana a tijera")
        (set `self.PlayerWins` true)
        (elif (and (== (`self.PlayerChoice`) 1) (== (`self.EnemyChoice`) 0))
          (`KismetSystemLibrary.PrintString` "Papel gana a Piedra")
          (set `self.PlayerWins` true)
          (elif (and (== (`self.PlayerChoice`) 2) (== (`self.EnemyChoice`) 1))
            (`KismetSystemLibrary.PrintString` "Tijera gana a papel")
            (set `self.PlayerWins` true))))
      (if (`self.PlayerWins`)
        (set `self.EnemyHealth` (- (`self.EnemyHealth`) (`self.DamagePerHit`)))
        (`KismetSystemLibrary.PrintString` (`KismetStringLibrary.Concat_StrStr` "¡¡¡JUGADOR GANA!!! - Jugador: " (`KismetStringLibrary.Conv_IntToString` (`self.PlayerHealth`)) " Enemigo: " (`KismetStringLibrary.Conv_IntToString` (`self.EnemyHealth`))) true true (struct :`G` 1.0 :`B` 0.002892 :`A` 1.0) 5.0)
        (else
          (set `self.PlayerHealth` (- (`self.PlayerHealth`) (`self.DamagePerHit`)))
          (`KismetSystemLibrary.PrintString` (`KismetStringLibrary.Concat_StrStr` "¡¡¡ENEMIGO GANA!!! - Jugador: " (`KismetStringLibrary.Conv_IntToString` (`self.PlayerHealth`)) " Enemigo: " (`KismetStringLibrary.Conv_IntToString` (`self.EnemyHealth`))) true true (struct :`R` 1.0 :`G` 0.010123 :`A` 1.0) 5.0)))
      (`self.CheckGameOver`))))

(fn `StartRound`
  (bind _returnvalue (`|CreateWidget` "/Game/Blueprints/WBP_RPS_UI.WBP_RPS_UI_C"))
  (`UserWidget.AddToViewport` _returnvalue 0)
  (`WidgetBlueprintLibrary.SetInputMode_UIOnlyEx` (`GameplayStatics.GetPlayerController` 0) _returnvalue))

(fn `UserConstructionScript`)